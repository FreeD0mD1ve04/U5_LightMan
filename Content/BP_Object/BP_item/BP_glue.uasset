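; BP_glue is an item that halts BP_Monster_overwatch monsters when a BP_TopDownCharacter overlaps its Capsule.
; It zeroes every such monster's walk speed and hides the Cube, disabling its collision.
; A five-second Delay inside the loop precedes resetting speed to a hard-coded value and destroying the item.
; Since that Delay ignores re-triggers, only the last monster in the array regains speed.
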(event OnComponentBeginOverlap(Capsule)
  (params (OverlappedComponent :type Primitive%20Component%20Object%20Reference) (OtherActor :type Actor%20Object%20Reference) (OtherComp :type Primitive%20Component%20Object%20Reference) (OtherBodyIndex :type Integer) (bFromSweep :type Boolean) (SweepResult :type Hit%20Result%20Structure%20%28by%20ref%29))
  (Utilities|Casting|CastToBP_TopDownCharacter OtherActor)
  (bind _outactors (Actor|GetAllActorsOfClass "/Game/BP_Object/BP_Monster/BP_Monster_overwatch.BP_Monster_overwatch_C"))
  (for _array_element _outactors
    (Variables|/Script/Engine.CharacterMovementComponent|SetMaxWalkSpeed (Variables|/Script/Engine.Character|GetCharacterMovement _array_element) 0.0)
    (Rendering|SetVisibility (Variables|Default|GetCube) false false)
    (Collision|SetCollisionEnabled (Variables|Default|GetCube) "NoCollision")
    (Utilities|FlowControl|Delay 5.0)
    (Variables|/Script/Engine.CharacterMovementComponent|SetMaxWalkSpeed (Variables|/Script/Engine.Character|GetCharacterMovement _array_element) 5e+02)
    (Actor|DestroyActor)))

(fn ConstructionScript)